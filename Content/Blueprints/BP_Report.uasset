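; BP_Report is a Blueprint that displays unit report data through a widget component, showing allied and enemy losses, retreat status and morale.
; DisplayReportData creates a new instance of the component's current widget class, assigns it and casts it to UW_UnitReport.
; It then passes in rounded loss totals, whether the unit has ever retreated, and average morale computed from the Report.
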(event EventDisplayReportData
  (bind _widget (Variables|Default|GetWidget))
  (bind _report (Variables|Default|GetReport))
  (bind (_alliedlosses _enemylosses _morale _bhaseverretreated) (Utilities|Struct|BreakUnitReport _report))
  (bind _returnvalue (UserInterface|CreateWidget (Utilities|GetClass (UserInterface|GetWidget _widget))))
  (UserInterface|SetWidget _widget _returnvalue)
  (bind _asuw_unit_report (Utilities|Casting|CastToUW_UnitReport _returnvalue))
  (Default|SetAlliedLosses _asuw_unit_report (Math|Float|Round _alliedlosses))
  (Default|SetEnemyLosses _asuw_unit_report (Math|Float|Round _enemylosses))
  (Default|SetRetreated _asuw_unit_report _bhaseverretreated)
  (Default|SetMorale _asuw_unit_report (Class|UnitReportFunctionLibrary|GetAverageMorale _report)))

(fn ConstructionScript)