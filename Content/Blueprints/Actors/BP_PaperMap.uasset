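; BP_PaperMap is a paper map actor that reports to the tutorial when game pieces are moved onto it.
; On BeginPlay it raises the paper mesh's translucent sort priority and caches the gameplay HUD.
; Its Box overlap checks for a CombatPiece or ScoutPiece and calls the matching map-overlap function on the HUD's Tutorial.
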(event OnComponentBeginOverlap(Box)
  (params (OverlappedComponent :type Primitive%20Component%20Object%20Reference) (OtherActor :type Actor%20Object%20Reference) (OtherComp :type Primitive%20Component%20Object%20Reference) (OtherBodyIndex :type Integer) (bFromSweep :type Boolean) (SweepResult :type Hit%20Result%20Structure%20%28by%20ref%29))
  (Utilities|Casting|CastToCombatPiece OtherActor
    (:then
      (Default|CombatMapOvelap (Variables|/Game/UI/BP_GameplayHUD.BP_GameplayHUD_C|GetTutorial (stale EventBeginPlay _asbp_gameplay_hud))))
    (:CastFailed
      (Utilities|Casting|CastToScoutPiece OtherActor)
      (Default|ScoutMapOvelap (Variables|/Game/UI/BP_GameplayHUD.BP_GameplayHUD_C|GetTutorial (stale EventBeginPlay _asbp_gameplay_hud))))))

(event EventBeginPlay
  (Rendering|SetTranslucentSortPriority (Variables|Default|GetPaperMeshComponent) 5)
  (bind _asbp_gameplay_hud (Utilities|Casting|CastToBP_GameplayHUD (HUD|GetHUD (Game|GetPlayerController 0)))))

(fn ConstructionScript)