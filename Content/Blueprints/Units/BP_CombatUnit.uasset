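; Combat unit Blueprint that shows a unit as six mesh components which disappear as it loses health.
; On BeginPlay or a CombatUnitData change, SetUnitMesh gives each component the data's mesh, adds its location and rotation offsets, and sets its scale.
; Tick polls CombatComponent health against fixed descending thresholds, hiding one more component at each, the last only below zero.
; Nothing in these graphs makes hidden components visible again.
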(event EventOnCombatUnitDataChange
  (Utilities|IsValid (Variables|/Script/Game1812.CombatUnitDataAsset|GetUnitMesh (Variables|Default|GetCombatUnitData))
    (:Is%20Valid
      (CallFunction|SetUnitMesh (Variables|Default|GetCube))
      (CallFunction|SetUnitMesh (Variables|Default|GetCube1))
      (CallFunction|SetUnitMesh (Variables|Default|GetCube2))
      (CallFunction|SetUnitMesh (Variables|Default|GetCube3))
      (CallFunction|SetUnitMesh (Variables|Default|GetCube4))
      (CallFunction|SetUnitMesh (Variables|Default|GetCube5)))))

(event EventBeginPlay
  (Utilities|IsValid (Variables|Default|GetCombatUnitData)
    (:Is%20Valid
      (Utilities|IsValid (Variables|/Script/Game1812.CombatUnitDataAsset|GetUnitMesh (Variables|Default|GetCombatUnitData))
        (:Is%20Valid
          (CallFunction|SetUnitMesh (Variables|Default|GetCube))
          (CallFunction|SetUnitMesh (Variables|Default|GetCube1))
          (CallFunction|SetUnitMesh (Variables|Default|GetCube2))
          (CallFunction|SetUnitMesh (Variables|Default|GetCube3))
          (CallFunction|SetUnitMesh (Variables|Default|GetCube4))
          (CallFunction|SetUnitMesh (Variables|Default|GetCube5)))))))

(event EventTick
  (params (DeltaSeconds :type Float%20%28single-precision%29))
  (bind _combatcomponent (Variables|Default|GetCombatComponent))
  (bind _healthpoints (Variables|/Script/Game1812.UnitCombatComponent|GetHealthPoints _combatcomponent))
  (if (< _healthpoints 8e+02)
    (Rendering|SetVisibility (Variables|Default|GetCube5) false false)
    (if (< _healthpoints 6e+02)
      (Rendering|SetVisibility (Variables|Default|GetCube4) false false)
      (if (< _healthpoints 4e+02)
        (Rendering|SetVisibility (Variables|Default|GetCube3) false false)
        (if (< _healthpoints 2e+02)
          (Rendering|SetVisibility (Variables|Default|GetCube2) false false)
          (if (< _healthpoints 1e+02)
            (Rendering|SetVisibility (Variables|Default|GetCube1) false false)
            (if (< _healthpoints 0.0)
              (Rendering|SetVisibility (Variables|Default|GetCube) false false))))))))

(fn ConstructionScript)

(fn SetUnitMesh
  (params (Component :type Static%20Mesh%20Component%20Object%20Reference))
  (bind _combatunitdata (Variables|Default|GetCombatUnitData))
  (bind _unitmeshtransform (Variables|/Script/Game1812.CombatUnitDataAsset|GetUnitMeshTransform _combatunitdata))
  (Components|StaticMesh|SetStaticMesh Component (Variables|/Script/Game1812.CombatUnitDataAsset|GetUnitMesh _combatunitdata))
  (Transformation|AddRelativeLocation Component (.location _unitmeshtransform) false false)
  (Transformation|AddRelativeRotation Component (.rotation _unitmeshtransform) false false)
  (Transformation|SetRelativeScale3D Component (.scale _unitmeshtransform)))