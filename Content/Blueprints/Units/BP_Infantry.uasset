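; BP_Infantry is an infantry unit drawn as six cube meshes that thin out as the unit loses health.
; On BeginPlay it applies the French material to every cube when Team is French Empire, with no other team handled.
; Each Tick it checks CombatComponent health against descending nested thresholds, hiding one more cube at each step until the last disappears below zero.
; Hidden cubes are never shown again.
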(event EventBeginPlay
  (switch Utilities|FlowControl|Switch|SwitchonETeam (Variables|Default|GetTeam)
    (:FRANCE
      (Rendering|Material|SetMaterial (Variables|Default|GetCube) 0 "/Game/Materials/M_French.M_French")
      (Rendering|Material|SetMaterial (Variables|Default|GetCube1) 0 "/Game/Materials/M_French.M_French")
      (Rendering|Material|SetMaterial (Variables|Default|GetCube2) 0 "/Game/Materials/M_French.M_French")
      (Rendering|Material|SetMaterial (Variables|Default|GetCube3) 0 "/Game/Materials/M_French.M_French")
      (Rendering|Material|SetMaterial (Variables|Default|GetCube4) 0 "/Game/Materials/M_French.M_French")
      (Rendering|Material|SetMaterial (Variables|Default|GetCube5) 0 "/Game/Materials/M_French.M_French"))))

(event Collision|EventActorBeginOverlap
  (params (OtherActor :type Actor%20Object%20Reference)))

(event EventTick
  (params (DeltaSeconds :type Float%20%28single-precision%29))
  (bind _combatcomponent (Variables|Default|GetCombatComponent))
  (bind _healthpoints (Variables|/Script/Game1812.CombatComponent|GetHealthPoints _combatcomponent))
  (if (< _healthpoints 8e+02)
    (Rendering|SetVisibility (Variables|Default|GetCube5) false false)
    (if (< _healthpoints 6e+02)
      (Rendering|SetVisibility (Variables|Default|GetCube4) false false)
      (if (< _healthpoints 4e+02)
        (Rendering|SetVisibility (Variables|Default|GetCube3) false false)
        (if (< _healthpoints 2e+02)
          (Rendering|SetVisibility (Variables|Default|GetCube2) false false)
          (if (< _healthpoints 1e+02)
            (Rendering|SetVisibility (Variables|Default|GetCube1) false false)
            (if (< _healthpoints 0.0)
              (Rendering|SetVisibility (Variables|Default|GetCube) false false))))))))

(fn ConstructionScript)