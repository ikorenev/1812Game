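; BP_GameState keeps a running count of elapsed seconds for the game and reports it to the player controller.
; On BeginPlay it starts a looping one-second timer, caches the first player's BP_PlayerController and sends it an initial zero.
; Each TimeIncrement call increments the Timer variable and passes the count to the controller's UpdateTimer, so no Tick logic is used.
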(event Custom|TimeIncrement
  (bind _result (Math|Integer|IncrementInt (Variables|Default|GetTimer))
    (:%20%20
      (Default|UpdateTimer (Variables|Default|GetPCrReference) _result))))

(event EventBeginPlay
  (Utilities|Time|SetTimerbyFunctionName 0 "TimeIncrement" 1.0 true)
  (bind _asbp_player_controller (Utilities|Casting|CastToBP_PlayerController (Game|GetPlayerController 0)))
  (Variables|Default|SetPCrReference _asbp_player_controller)
  (Default|UpdateTimer (Variables|Default|GetPCrReference)))

(event EventTick
  (params (DeltaSeconds :type Float%20%28single-precision%29)))

(fn ConstructionScript)