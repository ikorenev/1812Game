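; BP_ScoutPiece is the Scout game piece Blueprint, supplying that piece's sound effects.
; Sound events for drag start, selection, death and hit each play a sound at the actor's location.
; The hit event plays the placement sound only when the incoming force exceeds a squared threshold, filtering out weaker impacts.
; It contains no other active logic.
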(event EventPlaySoundDeath
  (Audio|PlaySoundatLocation "/Game/Audio/Sounds/Piece/SW_Death.SW_Death" (Transformation|GetActorLocation) "0, 0, 0" 1.0 1.0 0.0 0 0 0 0))

(event Collision|EventActorBeginOverlap
  (params (OtherActor :type Actor%20Object%20Reference)))

(event EventPlaySoundHit
  (params (Force :type Float%20%28single-precision%29))
  (if (> Force (Math|Float|Power 5e+03 2.0))
    (Audio|PlaySoundatLocation "/Game/Audio/Sounds/Piece/SW_Place.SW_Place" (Transformation|GetActorLocation) "0, 0, 0" 1.0 1.0 0.0 0 0 0 0)))

(event EventPlaySoundSelected
  (Audio|PlaySoundatLocation "/Game/Audio/Sounds/Piece/SW_Select.SW_Select" (Transformation|GetActorLocation) "0, 0, 0" 1.0 1.0 0.0 0 0 0 0))

(event EventPlaySoundStartDragging
  (Audio|PlaySoundatLocation "/Game/Audio/Sounds/Piece/SW_Drag.SW_Drag" (Transformation|GetActorLocation) "0, 0, 0" 1.0 1.0 0.0 0 0 0 0))

(event EventBeginPlay)

(event EventTick
  (params (DeltaSeconds :type Float%20%28single-precision%29)))

(fn ConstructionScript)