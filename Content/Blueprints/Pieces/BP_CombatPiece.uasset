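; BP_CombatPiece is a game piece for a combat unit that shows the unit's health on its foundation mesh.
; BeginPlay creates a dynamic instance of M_Health and applies it to the foundation mesh.
; Each Tick casts Unit to CombatUnit and sets the material's Percentage parameter to current HealthPoints divided by StartHP, polling rather than reacting to damage events.
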(event EventBeginPlay
  (bind _returnvalue (Rendering|Material|CreateDynamicMaterialInstance "/Game/Models/Materials/M_Health.M_Health" "None" "None" :!class /Script/Engine.KismetMaterialLibrary))
  (bind _output_get (Variables|Default|SetFoundationMaterial _returnvalue))
  (Rendering|Material|SetMaterial (Variables|Default|GetPieceFoundationMeshComponent) 0 _output_get))

(event Collision|EventActorBeginOverlap
  (params (OtherActor :type Actor%20Object%20Reference)))

(event EventTick
  (params (DeltaSeconds :type Float%20%28single-precision%29))
  (bind _ascombat_unit (Utilities|Casting|CastToCombatUnit (Variables|Default|GetUnit)))
  (Rendering|Material|SetScalarParameterValueonMaterials (Variables|Default|GetPieceFoundationMeshComponent) "Percentage" (/ (Variables|/Script/Game1812.CombatComponent|GetHealthPoints (Variables|/Script/Game1812.CombatUnit|GetCombatComponent _ascombat_unit)) (.starthp (Variables|/Script/Game1812.CombatUnit|GetCombatUnitStats _ascombat_unit)))))

(fn ConstructionScript)