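; Player controller that sets up the WB_SendOrders HUD and handles the pause menu.
; On BeginPlay it adds the HUD to the viewport, then pauses the game after a short delay.
; The PauseMenu input creates WB_PauseMenu once, reuses it, switches to UI-only input and pauses.
; UpdateTimer is an empty stub, with timer formatting and unit card creation left disconnected.
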(event Custom|UpdateTimer
  (params (Timer :type Integer))
  ;[1 1 1] Timer
  (Variables|Default|GetHUD
    (:then)
    (:else)))

(event Custom|CreateHUD
  ;[1 1 1] Create HUD in Gameplay
  (bind _returnvalue (UserInterface|CreateWidget "/Game/UI/Widgets/WB_SendOrders.WB_SendOrders_C"))
  (bind _output_get (Variables|Default|SetHUD _returnvalue))
  (UserInterface|Viewport|AddtoViewport _output_get 0)
  (Utilities|FlowControl|Delay 0.1)
  (Game|SetGamePaused true))

(event EventBeginPlay
  (CallFunction|CreateHUD)
  (CallFunction|UpdateTimer))

(event Input|ActionEvents|InputActionPauseMenu
  (params (Key :type Key%20Structure :default "None"))
  ;[1 1 1] Pause the game
  (:Pressed
    (Utilities|IsValid (Variables|Default|GetPauseMenuRef)
      (:Is%20Valid
        _)
      (:Is%20Not%20Valid
        (bind _returnvalue (UserInterface|CreateWidget "/Game/UI/Widgets/WB_PauseMenu.WB_PauseMenu_C"))
        (Variables|Default|SetPauseMenuRef _returnvalue)))
    (Input|SetInputModeUIOnly self (Variables|Default|GetPauseMenuRef) "DoNotLock" false)
    (UserInterface|Viewport|AddtoViewport (Variables|Default|GetPauseMenuRef) 0)
    (Game|SetGamePaused true)))

(event Input|MouseEvents|RightMouseButton
  (params (Key :type Key%20Structure :default "None")))

(fn ConstructionScript)